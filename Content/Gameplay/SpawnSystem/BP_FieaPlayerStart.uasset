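; BP_FieaPlayerStart is a tagged player start that previews in the editor which character its gameplay tag maps to.
; The construction script looks up the tag in TagToCharacterTypes, synchronously loads that class and copies its default object's skeletal mesh and materials onto a preview component.
; A text display shows the tag name in green, or a red error when the tag is unset or the character lookup fails.
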(event EventBeginPlay)

(event EventTick
  (params (DeltaSeconds :type Float%20%28single-precision%29)))

(fn ConstructionScript
  (Utilities|FlowControl|Sequence
    (:then_0
      (Construction|SetGoodTagText))
    (:then_1
      (Construction|LoadMesh))
    (:then_2
      (Construction|ConstructionShowTagText))))

(fn LoadMesh
  (bind _returnvalue (Utilities|LoadClassAssetBlocking (.Value (Utilities|Map|Find (Variables|Default|GetTagToCharacterTypes) (Variables|Tags|GetRegularGameplayTag)))))
  (bind _ascharacter (Utilities|Casting|CastToCharacterClass _returnvalue)
    (:then
      (bind _returnvalue_2 (Class|FIEAUtilityFunctionLibrary|GetClassCDO _ascharacter))
      (Utilities|FlowControl|Sequence
        (:then_0
          (Components|SkeletalMesh|SetSkeletalMeshAsset (Variables|Default|GetSkeletalMesh) (Variables|/Script/Engine.SkeletalMeshComponent|GetSkeletalMeshAsset (Variables|/Script/Engine.Character|GetMesh _returnvalue_2))))
        (:then_1
          (for (_array_element _array_index) (Rendering|Material|GetMaterials (Variables|/Script/Engine.Character|GetMesh _returnvalue_2))
            (Rendering|Material|SetMaterial (Variables|Default|GetSkeletalMesh) _array_index _array_element)))))
    (:CastFailed
      (Rendering|Components|TextRender|SetTextRenderColor (Variables|Default|GetDisplayText) (Math|Color|MakeColor 0 0 255))
      (Rendering|Components|TextRender|SetText (Variables|Default|GetDisplayText) (Utilities|Text|FormatText "ERROR: No Mesh for Tag")))))

(fn ConstructionShowTagText
  (if (== (Variables|Tags|GetRegularGameplayTag) "")
    (Rendering|Components|TextRender|SetTextRenderColor (Variables|Default|GetDisplayText) (Math|Color|MakeColor 0 0 255))
    (Rendering|Components|TextRender|SetText (Variables|Default|GetDisplayText) (Utilities|Text|FormatText "Please Set Tag"))))

(fn SetGoodTagText
  (Rendering|Components|TextRender|SetText (Variables|Default|GetDisplayText) (Utilities|Text|ToText(Name) (GameplayTags|GetTagName (Variables|Tags|GetRegularGameplayTag))))
  (Rendering|Components|TextRender|SetTextRenderColor (Variables|Default|GetDisplayText) (Math|Color|MakeColor 0 255 0)))

(fn QueriesYouCanDoonTags)