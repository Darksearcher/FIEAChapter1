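; Gameplay ability that teleports the avatar to a thrown translocator actor, supplied through SetTeleportActor.
; On activation it commits, clears the Thrown effect, plays a teleport cue and teleports, facing along the translocator's forward vector.
; A downward capsule trace sized to the character picks a safe destination against WorldStatic geometry.
; Success or failure, it destroys the translocator, then after a delay removes its input bindings and itself and ends.
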(event Ability|EventActivateAbility
  (|CallParentFunction)
  (bind _returnvalue (Ability|CommitAbility))
  (if _returnvalue
    (Utilities|FlowControl|Sequence
      (:then_0
        (Ability|RemoveGameplayEffectFromOwnerWithAssetTags "(GameplayTags=((TagName=\"Ability.Translocator.Thrown\")))"))
      (:then_1
        (GameplayCue|AddGameplayCue :GameplayCueTag "(TagName=\"GameplayCue.Ability.Teleport.Active\")"))
      (:then_2
        (bind _safeteleportlocation (CallFunction|FindSafeTeleportLocation))
        (bind _returnvalue_2 (Transformation|Teleport (.AvatarActor (Utilities|Struct|BreakGameplayAbilityActorInfo (Ability|GetActorInfo))) _safeteleportlocation (Math|Conversions|RotationFromXVector (Transformation|GetActorForwardVector (Variables|Default|GetMyTeleportActor)))))
        (if _returnvalue_2
          (Utilities|FlowControl|Sequence
            (:then_0
              (Actor|DestroyActor (Variables|Default|GetMyTeleportActor) :!label _label))
            (:then_1
              (Utilities|FlowControl|Delay 1.0 :!label _label_2)
              (CallFunction|RemoveAbility))
            (:then_2
              (Utilities|FlowControl|Delay 1.0 :!label _label_3)
              (Ability|EndAbility)))
          (else
            (Development|PrintString "ERROR: FAILED TO TP")
            (GameplayCue|RemoveGameplayCue "(TagName=\"GameplayCue.Ability.Teleport.Active\")")
            (Utilities|FlowControl|Sequence
              (:then_0
                (goto _label))
              (:then_1
                (goto _label_2))
              (:then_2
                (goto _label_3)))))))))

(event Ability|EventOnEndAbility
  (params (bWasCancelled :type Boolean)))

(fn SetTeleportActor
  (params (TeleportActor :type Actor%20Object%20Reference))
  (Variables|Default|SetMyTeleportActor TeleportActor))

(fn RemoveAbility
  (bind _asfieaability_system_component (Utilities|Casting|CastToFIEAAbilitySystemComponent (Ability|GetAbilitySystemComponentfromActorInfo)))
  (Class|FIEAAbilitySystemComponent|ClearAbilityBindings _asfieaability_system_component "/Game/Gameplay/InputMappingContext/InputActions/IA_TeleportTranslocator.IA_TeleportTranslocator")
  (bind _outabilityhandles (Class|AbilitySystemComponent|GetAllAbilities _asfieaability_system_component))
  (for _array_element _outabilityhandles
    (if (== (Utilities|GetClass (.ReturnValue (Ability|GameplayAbility|GetGameplayAbilityfromSpecHandle _asfieaability_system_component _array_element))) (Utilities|GetClass self))
      (Class|FIEAAbilitySystemComponent|ClearInputBinding _asfieaability_system_component _array_element)
      (GameplayAbilities|ClearAbility _asfieaability_system_component _array_element))))

(fn FindSafeTeleportLocation
  (bind _ascharacter (Utilities|Casting|CastToCharacter (.OwnerActor (Utilities|Struct|BreakGameplayAbilityActorInfo (Ability|GetActorInfo)))))
  (bind (_outhit _returnvalue) (Class|KismetSystemLibrary|CapsuleTraceSingleforObjects (+ (Transformation|GetActorLocation (Variables|Default|GetMyTeleportActor)) "0.000000,0.000000,100.000000") (Transformation|GetActorLocation (Variables|Default|GetMyTeleportActor)) (Components|Capsule|GetScaledCapsuleRadius (Variables|/Script/Engine.Character|GetCapsuleComponent _ascharacter)) (Components|Capsule|GetScaledCapsuleHalfHeight (Variables|/Script/Engine.Character|GetCapsuleComponent _ascharacter)) (Utilities|Array|MakeArray "ObjectTypeQuery1") false 0 "None" true))
  (if _returnvalue
    (return (.Location (Collision|BreakHitResult _outhit)))
    (else
      (return (Transformation|GetActorLocation (Variables|Default|GetMyTeleportActor))))))