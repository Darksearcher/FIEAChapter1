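; Gameplay Ability that throws a translocator projectile from the character's right hand.
; After committing, it plays the throw montage, listens for the GrenadeThrow notify tag, and ends when the montage completes, is interrupted or is cancelled.
; On that notify, a follow-camera trace picks the aim point, with a camera-forward fallback, and the projectile spawns with added upward pitch.
; The CanActivate override always returns true, ignoring the parent's result.
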(event Custom|GrenadeSpawn)

(event Ability|EventActivateAbility
  (|CallParentFunction)
  (bind _returnvalue (Ability|CommitAbility))
  (if _returnvalue
    (bind _asynctaskproxy (|FIEACreatePlayMontageandWaitforEvent "None" "/Game/Characters/Mannequins/Animations/Quinn/AM_Throw.AM_Throw" 1.0 "None" true 1.0 0.0 false)
      (:then
        (Variables|Default|SetMontageAsyncTask _asynctaskproxy)
        (EventDispatchers|BindEventtoOnNotifyBegin (Variables|Default|GetMontageAsyncTask) (EventDispatchers|CreateEvent :!event DelegateNotifyOccured)))
      (:OnCompleted
        (Ability|EndAbility))
      (:OnInterrupted
        (Ability|EndAbility))
      (:OnCancelled
        (Ability|EndAbility)))))

(event Ability|EventOnEndAbility
  (params (bWasCancelled :type Boolean))
  (|CallParentFunction bWasCancelled))

(event Ability|EventActivateAbilityFromEvent
  (params (EventData :type Gameplay%20Event%20Data%20Structure%20%28by%20ref%29))
  (|CallParentFunction EventData))

(fn K2CanActivateAbility
  (params (ActorInfo :type Gameplay%20Ability%20Actor%20Info%20Structure) (Handle :type Gameplay%20Ability%20Spec%20Handle%20Structure))
  (bind _relevanttags (|CallParentFunction ActorInfo Handle))
  (return _relevanttags true))

(fn DelegateNotifyOccured
  (params (TheNotify :type Gameplay%20Tag%20Structure))
  (if (GameplayTags|MatchesTag TheNotify "(TagName=\"Montage.Notify.Ability.GrenadeThrow\")" true)
    (Utilities|FlowControl|Sequence
      (:then_0
        (bind _asfieachapter_1character (Utilities|Casting|CastToFIEAChapter1Character (.AvatarActor (Utilities|Struct|BreakGameplayAbilityActorInfo (Ability|GetActorInfo))))
          (:then
            (LocalVariables|SetCurrentCamera (Variables|/Script/FIEAChapter1.FIEAChapter1Character|GetFollowCamera _asfieachapter_1character)))
          (:CastFailed
            (Development|PrintString "ERROR: NOT A FIEA CHARACTER????")
            (return))))
      (:then_1
        (bind (_outhit _returnvalue) (CallFunction|GetThrowDirection (LocalVariables|GetCurrentCamera)))
        (if _returnvalue
          (LocalVariables|SetCurrentHit _outhit)))
      (:then_2
        (CallFunction|SpawnTranslocatorinDirection (LocalVariables|GetCurrentHit) (LocalVariables|GetCurrentCamera))))))

(fn GetThrowDirection
  (params (FromCamera :type Camera%20Component%20Object%20Reference))
  (bind (_outhit _returnvalue) (Collision|LineTraceByChannel (Transformation|GetWorldLocation FromCamera) (+ (Transformation|GetWorldLocation FromCamera) (* (Math|Vector|GetForwardVector FromCamera) 3e+03)) "TraceTypeQuery1" false (Utilities|Array|MakeArray (.OwnerActor (Utilities|Struct|BreakGameplayAbilityActorInfo (Ability|GetActorInfo)))) "None"))
  (return _outhit _returnvalue))

(fn SpawnTranslocatorinDirection
  (params (HitDirection :type Hit%20Result%20Structure) (CameraBackUp :type Camera%20Component%20Object%20Reference))
  (bind _returnvalue (Ability|GetActorInfo))
  (bind _returnvalue_2 (Ability|GetActorInfo))
  (bind _owneractor (Utilities|Struct|BreakGameplayAbilityActorInfo _returnvalue_2))
  (bind _skeletalmeshcomponent (Utilities|Struct|BreakGameplayAbilityActorInfo _returnvalue))
  (bind _location (Collision|BreakHitResult HitDirection))
  (bind _returnvalue_3 (Transformation|GetWorldLocation CameraBackUp))
  (bind _returnvalue_4 (Math|Vector|GetForwardVector CameraBackUp))
  (bind _bblockinghit (Collision|BreakHitResult HitDirection))
  (bind _returnvalue_5 (Transformation|GetBoneTransform _skeletalmeshcomponent "hand_r" "RTS_World"))
  (bind _returnvalue_6 (* _returnvalue_4 1.5e+03))
  (bind _location_2 (Math|Transform|BreakTransform _returnvalue_5))
  (bind _returnvalue_7 (+ _returnvalue_6 _returnvalue_3))
  (bind _returnvalue_8 (Math|Vector|SelectVector _location _returnvalue_7 _bblockinghit))
  (bind _returnvalue_9 (- _returnvalue_8 _location_2))
  (bind _returnvalue_10 (Math|Conversions|RotationFromXVector _returnvalue_9))
  (bind (_roll _pitch _yaw) (Math|Rotator|BreakRotator _returnvalue_10))
  (bind _returnvalue_11 (Game|SpawnActorfromClass "/Game/Gameplay/BP/Projectiles/BP_Projectile_Translocator.BP_Projectile_Translocator_C" (Math|Transform|MakeTransform (.Location (Math|Transform|BreakTransform (Transformation|GetBoneTransform (.SkeletalMeshComponent (Utilities|Struct|BreakGameplayAbilityActorInfo (Ability|GetActorInfo))) "hand_r" "RTS_World"))) (Math|Rotator|MakeRotator _roll (+ _pitch 2e+01) _yaw)) "AlwaysSpawn" "MultiplyWithRoot" _owneractor (.AsPawn (Utilities|Casting|CastToPawn _owneractor))))
  (Variables|Default|SetTranslocatorThrown _returnvalue_11))