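; Base pickup actor that grants Gameplay Ability System effects to whatever overlaps it.
; On BeginPlay it binds a handler to the Box component's begin overlap.
; The pickup handler applies each valid effect in GEsToApply to the other actor's Ability System Component at level zero.
; It then destroys the pickup, with no filtering of the overlapping actor.
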(event EventBeginPlay
  (Collision|BindEventtoOnComponentBeginOverlap (Variables|Default|GetBox) (EventDispatchers|CreateEvent :!event DelegateonPickup)))

(event Collision|EventActorBeginOverlap
  (params (OtherActor :type Actor%20Object%20Reference)))

(event EventTick
  (params (DeltaSeconds :type Float%20%28single-precision%29)))

(fn ConstructionScript)

(fn DelegateonPickup
  (params (OverlappedComponent :type Primitive%20Component%20Object%20Reference) (OtherActor :type Actor%20Object%20Reference) (OtherComp :type Primitive%20Component%20Object%20Reference) (OtherBodyIndex :type Integer) (bFromSweep :type Boolean) (SweepResult :type Hit%20Result%20Structure%20%28by%20ref%29))
  (for _array_element (Variables|Default|GetGEsToApply)
    (LocalVariables|SetCurrentGE _array_element)
    (LocalVariables|GetCurrentGE
      (:then
        (GameplayEffects|ApplyGameplayEffectToSelf (Ability|GetAbilitySystemComponent OtherActor) (LocalVariables|GetCurrentGE) 0.0 (Utilities|Struct|MakeGameplayEffectContextHandle)))
      (:else)))
  (Actor|DestroyActor))