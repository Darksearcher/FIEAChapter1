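; Foot FX actor component meant for Characters, spawning a Niagara effect at a supplied location.
; Setter and clear functions control the stored Niagara system, which PlaySFXAtLocation spawns at the passed location.
; Despite the SFX naming, it handles only Niagara effects and plays no sound.
; BeginPlay prints an error if the owner is not a Character; Tick is unused.
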(event EventBeginPlay
  (Utilities|Casting|CastToCharacter (Components|GetOwner)
    (:CastFailed
      (Development|PrintString "ERROR: Why is this not on a character"))))

(event EventTick
  (params (DeltaSeconds :type Float%20%28single-precision%29)))

(fn PlaySFXatLocation
  (params (LocationToPlay :type Vector))
  (Niagara|SpawnSystematLocation (Variables|Default|GetNiagaraSystemToPlay) LocationToPlay))

(fn SetSFXtoPlay
  (params (SFXToPlay :type Niagara%20System%20Object%20Reference))
  (Variables|Default|SetNiagaraSystemToPlay SFXToPlay))

(fn ClearFXtoPlay
  (Variables|Default|SetNiagaraSystemToPlay 0))