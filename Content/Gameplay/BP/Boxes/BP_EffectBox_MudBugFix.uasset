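; BP_EffectBox_MudBugFix is a child effect box, likely for mud, that catches actors removing their boots while inside it.
; When WithBugFix is set and an overlapping actor has the Equipped.Boots gameplay tag, a looping timer starts.
; The timer polls the box's overlapping actors, re-running the overlap handler for any ability-system actor lacking the tag and clearing itself.
; It also stops when the box is empty.
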(event EventBeginPlay
  (|CallParentFunction) ; This node is disabled and will not be called.\nDrag off pins to build functionality.
)

(event Collision|EventActorBeginOverlap
  (params (OtherActor :type Actor%20Object%20Reference))
  (|CallParentFunction OtherActor) ; This node is disabled and will not be called.\nDrag off pins to build functionality.
)

(event EventTick
  (params (DeltaSeconds :type Float%20%28single-precision%29))
  (|CallParentFunction DeltaSeconds) ; This node is disabled and will not be called.\nDrag off pins to build functionality.
)

(fn ConstructionScript
  (|CallParentFunction))

(fn DelegateonOverlap
  (params (OverlappedComponent :type Primitive%20Component%20Object%20Reference) (OtherActor :type Actor%20Object%20Reference) (OtherComp :type Primitive%20Component%20Object%20Reference) (OtherBodyIndex :type Integer) (bFromSweep :type Boolean) (SweepResult :type Hit%20Result%20Structure%20%28by%20ref%29))
  (bind _returnvalue (Ability|GetAbilitySystemComponent OtherActor))
  (|CallParentFunction OverlappedComponent OtherActor OtherComp OtherBodyIndex bFromSweep SweepResult)
  (if (Variables|Default|GetWithBugFix)
    (Utilities|IsValid _returnvalue
      (:Is%20Valid
        (if (GameplayTags|HasMatchingGameplayTag _returnvalue "(TagName=\"CharacterState.Equipped.Boots\")")
          (bind _returnvalue_2 (Utilities|Time|SetTimerbyEvent (EventDispatchers|CreateEvent :!event DelegateBootTimerCheck) 0.3 true))
          (Variables|Default|SetBootCheckTImer _returnvalue_2)
          (return))))))

(fn DelegateBootTimerCheck
  (Utilities|FlowControl|Sequence
    (:then_0
      (LocalVariables|SetCurrentOverlappingActors (Collision|GetOverlappingActors (Variables|Default|GetBox) 0 :!class /Script/Engine.PrimitiveComponent)))
    (:then_1
      (if (Utilities|Array|IsEmpty (LocalVariables|GetCurrentOverlappingActors))
        (Utilities|Time|ClearandInvalidateTimerbyHandle (Variables|Default|GetBootCheckTImer))
        (return)))
    (:then_2
      (for _array_element (LocalVariables|GetCurrentOverlappingActors)
        (LocalVariables|SetGetCurrentOverlapActor _array_element)
        (LocalVariables|SetGetLocalAbilitySystemComponent (Ability|GetAbilitySystemComponent _array_element))
        (LocalVariables|GetGetLocalAbilitySystemComponent
          (:then
            (Utilities|IsValid (LocalVariables|GetGetLocalAbilitySystemComponent)
              (:Is%20Valid
                (if (not (GameplayTags|HasMatchingGameplayTag (LocalVariables|GetGetLocalAbilitySystemComponent) "(TagName=\"CharacterState.Equipped.Boots\")"))
                  (CallFunction|DelegateonOverlap 0 (LocalVariables|GetGetCurrentOverlapActor) 0 0 false)
                  (Utilities|Time|ClearandInvalidateTimerbyHandle (Variables|Default|GetBootCheckTImer))))))
          (:else))))))