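; BP_EffectBox is a box volume that grants Gameplay Ability System effects to actors while they overlap it.
; On BeginPlay it binds the box's begin and end overlap events.
; Entry applies the first valid effect in GEsToApply to the actor's ability system and records its handle in ActiveGEs.
; Exit ignores those handles, removing all stacks of every listed effect by class, with the actor as instigator.
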(event EventBeginPlay
  (Utilities|FlowControl|Sequence
    (:then_0
      (Collision|BindEventtoOnComponentBeginOverlap (Variables|Default|GetBox) (EventDispatchers|CreateEvent :!event DelegateonOverlap)))
    (:then_1
      (Collision|BindEventtoOnComponentEndOverlap (Variables|Default|GetBox) (EventDispatchers|CreateEvent :!event DelegateonEndOverlap)))))

(event Collision|EventActorBeginOverlap
  (params (OtherActor :type Actor%20Object%20Reference)))

(event EventTick
  (params (DeltaSeconds :type Float%20%28single-precision%29)))

(fn ConstructionScript)

(fn DelegateonOverlap
  (params (OverlappedComponent :type Primitive%20Component%20Object%20Reference) (OtherActor :type Actor%20Object%20Reference) (OtherComp :type Primitive%20Component%20Object%20Reference) (OtherBodyIndex :type Integer) (bFromSweep :type Boolean) (SweepResult :type Hit%20Result%20Structure%20%28by%20ref%29))
  (for _array_element (Variables|Ability|GetGEsToApply)
    (LocalVariables|SetCurrentGE _array_element)
    (LocalVariables|GetCurrentGE
      (:then
        (if (Utilities|IsValidClass (LocalVariables|GetCurrentGE))
          (bind _returnvalue (GameplayEffects|ApplyGameplayEffectToSelf (Ability|GetAbilitySystemComponent OtherActor) (LocalVariables|GetCurrentGE) 0.0 (Utilities|Struct|MakeGameplayEffectContextHandle)))
          (Utilities|Array|Add (Variables|Ability|GetActiveGEs) _returnvalue)
          (return)))
      (:else))))

(fn DelegateonEndOverlap
  (params (OverlappedComponent :type Primitive%20Component%20Object%20Reference) (OtherActor :type Actor%20Object%20Reference) (OtherComp :type Primitive%20Component%20Object%20Reference) (OtherBodyIndex :type Integer))
  (bind _returnvalue (Ability|GetAbilitySystemComponent OtherActor))
  (for _array_element (Variables|Ability|GetGEsToApply)
    (GameplayEffects|RemoveActiveGameplayEffectbySourceEffect _returnvalue _array_element _returnvalue -1)))